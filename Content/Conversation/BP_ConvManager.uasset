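; Conversation manager actor that runs NPC dialogue, either as plain text or alongside a Level Sequence cutscene.
; StartConv shows the conversation widget at a given row; Sequence mode first loads the sequence and cut frame numbers from a data table.
; Space or gamepad bottom button writes the next line and jumps the sequencer to the next cut frame.
; Input re-enables after each line; EndConv stops the sequence and destroys the actor.
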(event `Key|Gamepad_FaceButton_Bottom`
  (params (Key :type "Key Structure"))
  (bind _is_sequence (`self.Is Sequence`))
  (:`Pressed`
    (`/Game/Conversation/BPI_Conversation.StartWrite` (`self.W_Conv`) _is_sequence :!label _label) ; 次の行へ
    (`self.DisableInput` (`GameplayStatics.GetPlayerController` 0))
    (if _is_sequence
      (if (< (`self.CurrentCutNum`) (`KismetArrayLibrary.Array_Length` (`self.CutFrameNums`)))
        (`self.NextCutScene`)
        (else
          (`KismetSystemLibrary.PrintString` "終わり！！！！！！！！！！！！！１１１"))))))

(event `self.ReceiveBeginPlay`
  (bind _returnvalue (`|CreateWidget` "/Game/Conversation/WBP_Conversation.WBP_Conversation_C"))
  (set `self.W_Conv` _returnvalue))

(event `Key|SpaceBar`
  (params (Key :type "Key Structure"))
  (:`Pressed`
    (goto _label)))

(event `/Game/Conversation/BPI_Conversation.EndOneLine`
  (`KismetSystemLibrary.Delay` 1.0)
  (`self.EnableInput` (`GameplayStatics.GetPlayerController` 0))
  (`KismetSystemLibrary.PrintString` "入力を許可"))

(event `/Game/Conversation/BPI_Conversation.StartConv`
  (params (`NormalConv?` :type "/Game/Conversation/E_ConvType Enum" :default "NewEnumerator0") (RowNum :type Integer) (SeqName :type Name))
  (bind _w_conv (`self.W_Conv`))
  (bind _cutframenums (`self.CutFrameNums`))
  ;[1 1 1] 会話開始時のイベント（From BP_NPC）
  (switch `/Game/Conversation/E_ConvType` `NormalConv?`
    (:`NewEnumerator0`
      (set `/Game/Conversation/WBP_Conversation.RowNum` RowNum _w_conv :!label _label_2) ; 先にセット
      (`UserWidget.AddToViewport` _w_conv 0) ; アニメーション付けるならこれの後ろに
      (`self.DisableInput` (`GameplayStatics.GetPlayerController` 0)))
    (:`NewEnumerator4`
      (bind _returnvalue (`|GetDataTableRow` "/Game/Conversation/DT_SeqConvCSV.DT_SeqConvCSV" SeqName)
        (:`then`
          (`|ExecutionSequence`
            (:`then_0`
              (bind (_outactor _returnvalue_2) (`LevelSequencePlayer.CreateLevelSequencePlayer` (`.LevelSequence_6_3211F7EF4F820F5C88C57B89FAE85AA8` (break `/Game/Conversation/S_SeqConv` _returnvalue)) (make `MovieSceneSequencePlaybackSettings` true (struct) 1.0 0.0 false false true true true))) ; LevelSequenceは無駄参照防止のために仲介人いれる\n複数ならDataTableを使うといいかも
              (set `self.SeqPlayer` _returnvalue_2)
              (set `self.Is Sequence` true))
            (:`then_1`
              (`KismetArrayLibrary.Array_Clear` _cutframenums) ; 再利用できるように
              (set `self.CurrentCutNum` 0)
              (for _array_element (`.CutFrameNums_15_DCDF784D4DC9AEA57DB9A6BD819A9B63` (break `/Game/Conversation/S_SeqConv` _returnvalue))
                (`KismetArrayLibrary.Array_Add` _cutframenums _array_element))
              (goto _label_2))))))))

(event `/Game/Conversation/BPI_Conversation.EndConv`
  ;[1 1 1] 会話の終了 (From WBP_Conversation)
  (`MovieSceneSequencePlayer.Stop` (`self.SeqPlayer`))
  (`self.EnableInput` (`GameplayStatics.GetPlayerPawn` 0) (`GameplayStatics.GetPlayerController` 0))
  (`self.K2_DestroyActor`))

(fn `NextCutScene`
  (bind _seqplayer (`self.SeqPlayer`))
  (bind _output (`|GetArrayItem` (`self.CutFrameNums`) (`self.CurrentCutNum`)))
  (`|ExecutionSequence`
    (:`then_0`
      (`KismetSystemLibrary.PrintString` (`KismetStringLibrary.Conv_IntToString` _output)))
    (:`then_1`
      (`MovieSceneSequencePlayer.SetPlaybackPosition` _seqplayer (make `MovieSceneSequencePlaybackParams` (make `FrameTime` (make `FrameNumber` _output)) 0.0 "" "Frame" "Jump" true))
      (`MovieSceneSequencePlayer.Play` _seqplayer) ; シーケンサーを再開する
      (`/Engine/EditorBlueprintResources/StandardMacros.IncrementInt` (`self.CurrentCutNum`)) ; ※後に更新
    )))

(fn `UserConstructionScript`)
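; Utility actor that generates comma-separated character status text on BeginPlay, apparently as table data for levels 1 to 100.
; It seeks seven stat timelines (HP, MP, Attack, Defense, Speed, SpellPower, Luck) to each index, using them as growth curves through nested Update outputs.
; Floored values and two default all-False element maps are appended after the Status prefix, printed and saved to a BP_StatusExportSaveGame slot.
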(event `self.ReceiveBeginPlay`
  (`GameplayStatics.DoesSaveGameExist` (`self.StatusSaveGame`))
  (bind _returnvalue (`GameplayStatics.CreateSaveGameObject` "/Game/GameData/BP_StatusExportSaveGame.BP_StatusExportSaveGame_C"))
  (set `self.SaveGame` _returnvalue)
  (`self.StatusTextSet`))

(event `Key|One`
  (params (Key :type "Key Structure")))

(event `Key|Zero` :paused true
  (params (Key :type "Key Structure")))

(event `StatusTextSet`
  (bind _savegame (`self.SaveGame`))
  (bind _returnvalue (`KismetStringLibrary.Concat_StrStr` (`self.Status`) " \n" (`self.KeepStatusString`)))
  (for _index (range 1 101)
    (bind _returnvalue_2 (`KismetMathLibrary.Conv_IntToDouble` _index))
    (bind (_direction _hp) (`Timeline|HPGraph` :`NewTime` _returnvalue_2 :!via `SetNewTime`)
      (:`Update`
        (bind (_direction_2 _mp) (`Timeline|MPGraph` :`NewTime` _returnvalue_2 :!via `SetNewTime`)
          (:`Update`
            (bind (_direction_3 _attack) (`Timeline|AttackGraph` :`NewTime` _returnvalue_2 :!via `SetNewTime`)
              (:`Update`
                (bind (_direction_4 _defense) (`Timeline|DefenseGraph` :`NewTime` _returnvalue_2 :!via `SetNewTime`)
                  (:`Update`
                    (bind (_direction_5 _speed) (`Timeline|SpeedGraph` :`NewTime` _returnvalue_2 :!via `SetNewTime`)
                      (:`Update`
                        (bind (_direction_6 _spellpowe) (`Timeline|SpellPowerGraph` :`NewTime` _returnvalue_2 :!via `SetNewTime`)
                          (:`Update`
                            (bind (_direction_7 _luck) (`Timeline|LuckGraph` :`NewTime` _returnvalue_2 :!via `SetNewTime`)
                              (:`Update`
                                (set `self.KeepStatusString` (`KismetStringLibrary.Concat_StrStr` (`KismetStringLibrary.Concat_StrStr` (`KismetStringLibrary.Concat_StrStr` (`KismetStringLibrary.Concat_StrStr` (`KismetStringLibrary.Concat_StrStr` (`KismetStringLibrary.Concat_StrStr` (`KismetStringLibrary.Concat_StrStr` (`KismetStringLibrary.Concat_StrStr` (`KismetStringLibrary.Concat_StrStr` (`self.KeepStatusString`) (`KismetStringLibrary.Conv_IntToString` _index) ",") "\"" (`KismetStringLibrary.Conv_IntToString` (`KismetMathLibrary.FFloor` _hp)) "\"" ",") "\"" (`KismetStringLibrary.Conv_IntToString` (`KismetMathLibrary.FFloor` _mp)) "\"" ",") "\"" (`KismetStringLibrary.Conv_IntToString` (`KismetMathLibrary.FFloor` _attack)) "\"" ",") "\"" (`KismetStringLibrary.Conv_IntToString` (`KismetMathLibrary.FFloor` _defense)) "\"" ",") "\"" (`KismetStringLibrary.Conv_IntToString` (`KismetMathLibrary.FFloor` _speed)) "\"" ",") "\"" (`KismetStringLibrary.Conv_IntToString` (`KismetMathLibrary.FFloor` _spellpowe)) "\"" ",") "\"" (`KismetStringLibrary.Conv_IntToString` (`KismetMathLibrary.FFloor` _luck)) "\"" ",") "\"((Fire, False),(Water, False),(Thunder, False),(Earth, False),(Dark, False),(Light, False),(Normal, False))\",\"((Fire, False),(Water, False),(Thunder, False),(Earth, False),(Dark, False),(Light, False),(Normal, False))\"" " \n")))))))))))))))))
  (`KismetSystemLibrary.PrintString` _returnvalue true true (struct :`G` 0.66 :`B` 1.0 :`A` 1.0) 10.0)
  (set `/Game/GameData/BP_StatusExportSaveGame.StatusText` (`KismetTextLibrary.Conv_StringToText` _returnvalue) _savegame)
  (`GameplayStatics.SaveGameToSlot` _savegame (`self.StatusSaveGame`)))

(fn `UserConstructionScript`)